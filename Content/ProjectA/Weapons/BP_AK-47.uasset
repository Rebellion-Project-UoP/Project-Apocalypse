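; AK-47 weapon Blueprint for crafting-table customisation, built from modular parts.
; On BeginPlay it attaches barrel, grip, magazine, stock and scope to named sockets on the weapon body.
; Clicking the barrel or magazine toggles that part's list widget, closes other part widgets and passes the parent actor as CraftingTable.
; Hover events only print part names; grip, stock and scope have no click handlers, and the barrel extension attach is unconnected.
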(event `self.ReceiveBeginPlay`
  (`parent.ReceiveBeginPlay`)
  (`SceneComponent.K2_AttachToComponent` (`self.WeaponBarrel`) (`self.WeaponBody`) "Barrel-Slot" "KeepRelative" "KeepRelative" "KeepRelative" true)
  (`SceneComponent.K2_AttachToComponent` (`self.WeaponGrip`) (`self.WeaponBody`) "Grip-Slot" "KeepRelative" "KeepRelative" "KeepRelative" true)
  (`SceneComponent.K2_AttachToComponent` (`self.WeaponMagazine`) (`self.WeaponBody`) "Mag-Slot" "KeepRelative" "KeepRelative" "KeepRelative" true)
  (`SceneComponent.K2_AttachToComponent` (`self.WeaponStock`) (`self.WeaponBody`) "Stock-Slot" "KeepRelative" "KeepRelative" "KeepRelative" true)
  (`SceneComponent.K2_AttachToComponent` (`self.WeaponScope`) (`self.WeaponBody`) "Scope-Slot" "KeepRelative" "KeepRelative" "KeepRelative" true))

(event `self.ReceiveTick`
  (params (DeltaSeconds :type "Float (single-precision)"))
  (`parent.ReceiveTick` DeltaSeconds))

(event `self.WeaponBody.OnBeginCursorOver`
  (params (TouchedComponent :type "PrimitiveComponent Object Reference"))
  ;[1 0.9055 0.2271] Weapon Table customisation
  (`KismetSystemLibrary.PrintString` "Body"))

(event `self.WeaponScope.OnBeginCursorOver`
  (params (TouchedComponent :type "PrimitiveComponent Object Reference"))
  ;[1 0.9055 0.2271] Weapon Table customisation
  (`KismetSystemLibrary.PrintString` "Scope"))

(event `self.WeaponStock.OnBeginCursorOver`
  (params (TouchedComponent :type "PrimitiveComponent Object Reference"))
  ;[1 0.9055 0.2271] Weapon Table customisation
  (`KismetSystemLibrary.PrintString` "Stock"))

(event `self.WeaponBarrel.OnBeginCursorOver`
  (params (TouchedComponent :type "PrimitiveComponent Object Reference"))
  ;[1 0.9055 0.2271] Weapon Table customisation
  (`KismetSystemLibrary.PrintString` "Barrel"))

(event `self.WeaponGrip.OnBeginCursorOver`
  (params (TouchedComponent :type "PrimitiveComponent Object Reference"))
  ;[1 0.9055 0.2271] Weapon Table customisation
  (`KismetSystemLibrary.PrintString` "Grip"))

(event `self.WeaponBarrel.OnClicked`
  (params (TouchedComponent :type "PrimitiveComponent Object Reference") (ButtonPressed :type "Key Structure"))
  ;[1 0.9055 0.2271] Weapon Table customisation
  (`/Engine/EditorBlueprintResources/StandardMacros.IsValid` (`self.WBP_Barrel`)
    (:`Is Valid`
      (`Widget.RemoveFromParent` (`self.WBP_Barrel`))
      (set `self.WBP_Barrel` null))
    (:`Is Not Valid`
      (bind _returnvalue (`|CreateWidget` "/Game/ProjectA/UI/WeaponCrafting/WBP_BarrelList_AK47.WBP_BarrelList_AK47_C"))
      (bind _output_get (set `self.WBP_Barrel` _returnvalue))
      (`self.RemoveOtherWidgets` _output_get)
      (bind _aswbp_barrel_list_ak47 (cast `/Game/ProjectA/UI/WeaponCrafting/WBP_BarrelList_AK47` (`self.WBP_Barrel`)))
      (set `/Game/ProjectA/UI/WeaponCrafting/WBP_BarrelList_AK47.CraftingTable` (`self.GetParentActor`) _aswbp_barrel_list_ak47)
      (`UserWidget.AddToViewport` (`self.WBP_Barrel`) 0))))

(event `self.WeaponMagazine.OnClicked`
  (params (TouchedComponent :type "PrimitiveComponent Object Reference") (ButtonPressed :type "Key Structure"))
  ;[1 0.9055 0.2271] Weapon Table customisation
  (`/Engine/EditorBlueprintResources/StandardMacros.IsValid` (`self.WBP_Magazine`)
    (:`Is Valid`
      (`Widget.RemoveFromParent` (`self.WBP_Magazine`))
      (set `self.WBP_Magazine` null))
    (:`Is Not Valid`
      (bind _returnvalue (`|CreateWidget` "/Game/ProjectA/UI/WeaponCrafting/WBP_MagazineList_AK47.WBP_MagazineList_AK47_C"))
      (bind _output_get (set `self.WBP_Magazine` _returnvalue))
      (`self.RemoveOtherWidgets` _output_get)
      (bind _aswbp_magazine_list_ak47 (cast `/Game/ProjectA/UI/WeaponCrafting/WBP_MagazineList_AK47` (`self.WBP_Magazine`)))
      (set `/Game/ProjectA/UI/WeaponCrafting/WBP_MagazineList_AK47.CraftingTable` (`self.GetParentActor`) _aswbp_magazine_list_ak47)
      (`UserWidget.AddToViewport` (`self.WBP_Magazine`) 0))))

(event `self.WeaponMagazine.OnBeginCursorOver`
  (params (TouchedComponent :type "PrimitiveComponent Object Reference"))
  ;[1 0.9055 0.2271] Weapon Table customisation
  (`KismetSystemLibrary.PrintString` "Magazine"))

(fn `RemoveOtherWidgets`
  (params (DesiredWidget :type "UserWidget Object Reference"))
  (`|ExecutionSequence`
    (:`then_0`
      (if (not (== (`self.WBP_Magazine`) (`local.DesiredWidget`)))
        (`/Engine/EditorBlueprintResources/StandardMacros.IsValid` (`self.WBP_Magazine`)
          (:`Is Valid`
            (`Widget.RemoveFromParent` (`self.WBP_Magazine`))
            (set `self.WBP_Magazine` null)))))
    (:`then_1`
      (if (not (== (`self.WBP_Barrel`) (`local.DesiredWidget`)))
        (`/Engine/EditorBlueprintResources/StandardMacros.IsValid` (`self.WBP_Barrel`)
          (:`Is Valid`
            (`Widget.RemoveFromParent` (`self.WBP_Barrel`))
            (set `self.WBP_Barrel` null)))))
    (:`then_2`
      (if (not (== (`self.WBP_BarrelExtension`) (`local.DesiredWidget`)))
        (`/Engine/EditorBlueprintResources/StandardMacros.IsValid` (`self.WBP_BarrelExtension`)
          (:`Is Valid`
            (`Widget.RemoveFromParent` (`self.WBP_BarrelExtension`))
            (set `self.WBP_BarrelExtension` null)))))
    (:`then_3`
      (if (not (== (`self.WBP_Grip`) (`local.DesiredWidget`)))
        (`/Engine/EditorBlueprintResources/StandardMacros.IsValid` (`self.WBP_Grip`)
          (:`Is Valid`
            (`Widget.RemoveFromParent` (`self.WBP_Grip`))
            (set `self.WBP_Grip` null)))))
    (:`then_4`
      (if (not (== (`self.WBP_Stock`) (`local.DesiredWidget`)))
        (`/Engine/EditorBlueprintResources/StandardMacros.IsValid` (`self.WBP_Stock`)
          (:`Is Valid`
            (`Widget.RemoveFromParent` (`self.WBP_Stock`))
            (set `self.WBP_Stock` null)))))
    (:`then_5`
      (if (not (== (`self.WBP_Scope`) (`local.DesiredWidget`)))
        (`/Engine/EditorBlueprintResources/StandardMacros.IsValid` (`self.WBP_Scope`)
          (:`Is Valid`
            (`Widget.RemoveFromParent` (`self.WBP_Scope`))
            (set `self.WBP_Scope` null)))))))

(fn `UserConstructionScript`
  (`parent.UserConstructionScript`))